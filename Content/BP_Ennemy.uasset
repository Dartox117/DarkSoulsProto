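; BP_Ennemy is a melee enemy that faces the player, attacks in range and takes damage.
; Rotate and AttackRange overlaps set flags that Tick reads to yaw the mesh toward the player controller's focal location and play a light attack montage with a post-attack cooldown.
; AnyDamage lowers and prints Health, playing a slowed knockdown below zero, then restoring health when it completes.
; GetCurrentHealth, GetMaxHealth and TakeDamage are empty stubs.
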(event OnComponentBeginOverlap(Rotate)
  (params (OverlappedComponent :type Primitive%20Component%20Object%20Reference) (OtherActor :type Actor%20Object%20Reference) (OtherComp :type Primitive%20Component%20Object%20Reference) (OtherBodyIndex :type Integer) (bFromSweep :type Boolean) (SweepResult :type Hit%20Result%20Structure%20%28by%20ref%29))
  (Variables|Default|SetNeedToLook true))

(event OnComponentEndOverlap(Rotate)
  (params (OverlappedComponent :type Primitive%20Component%20Object%20Reference) (OtherActor :type Actor%20Object%20Reference) (OtherComp :type Primitive%20Component%20Object%20Reference) (OtherBodyIndex :type Integer))
  (Variables|Default|SetNeedToLook false))

(event OnComponentBeginOverlap(AttackRange)
  (params (OverlappedComponent :type Primitive%20Component%20Object%20Reference) (OtherActor :type Actor%20Object%20Reference) (OtherComp :type Primitive%20Component%20Object%20Reference) (OtherBodyIndex :type Integer) (bFromSweep :type Boolean) (SweepResult :type Hit%20Result%20Structure%20%28by%20ref%29))
  (Variables|Default|SetNeedToAttack true))

(event OnComponentEndOverlap(AttackRange)
  (params (OverlappedComponent :type Primitive%20Component%20Object%20Reference) (OtherActor :type Actor%20Object%20Reference) (OtherComp :type Primitive%20Component%20Object%20Reference) (OtherBodyIndex :type Integer))
  (Variables|Default|SetNeedToAttack false))

(event Game|Damage|EventAnyDamage
  (params (Damage :type Float%20%28single-precision%29) (DamageType :type Damage%20Type%20Object%20Reference) (InstigatedBy :type Controller%20Object%20Reference) (DamageCauser :type Actor%20Object%20Reference))
  (if (Variables|Default|GetCanTakeDamage)
    (bind _output_get (Variables|Default|SetHealth (- (Variables|Default|GetHealth) Damage)))
    (Development|PrintString (Utilities|String|ToString(Float) _output_get))
    (if (< (Variables|Default|GetHealth) 0.0)
      (Animation|Montage|PlayMontage (Variables|Default|GetSkeletalMesh) "/Game/Sword_Animations/Animations/Sequence1/08_Hit/10_Knock_Down/Knock_Down_Start_Seq_Montage.Knock_Down_Start_Seq_Montage" 0.5
        (:OnCompleted
          (Variables|Default|SetHealth 5e+02)
          (Variables|Default|SetCanTakeDamage true))))))

(event EventTick
  (params (DeltaSeconds :type Float%20%28single-precision%29))
  (bind _returnvalue (Game|GetPlayerController 0))
  (bind _skeletalmesh (Variables|Default|GetSkeletalMesh))
  (bind _returnvalue_2 (Transformation|GetWorldLocation _skeletalmesh))
  (bind _returnvalue_3 (Class|PlayerController|GetFocalLocation _returnvalue))
  (bind _returnvalue_4 (Math|Rotator|FindLookatRotation _returnvalue_2 _returnvalue_3))
  (if (Variables|Default|GetNeedToLook)
    (Transformation|SetWorldRotation (Variables|Default|GetSkeletalMesh) (Math|Rotator|MakeRotator (.roll _returnvalue_4) 0.0 (- (.yaw _returnvalue_4) 9e+01)) false false)
    (if (Variables|Default|GetNeedToAttack)
      (if (not (Variables|Default|GetIsAttacking))
        (Variables|Default|SetIsAttacking true)
        (Animation|Montage|PlayMontage (Variables|Default|GetSkeletalMesh) "/Game/Sword_Animations/Animations/Sequence1/02_Attack/03_Combo_Attack_03/Light_Attack_Montage.Light_Attack_Montage"
          (:OnCompleted
            (Utilities|FlowControl|Delay 5.0)
            (Variables|Default|SetIsAttacking false)))))))

(fn ConstructionScript)

(fn GetCurrentHealth
  (return 0.0))

(fn GetMaxHealth
  (return 0.0))

(fn TakeDamage
  (params (DamageAmount :type Float%20%28double-precision%29))
  (return))